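; Melee enemy AI that chases the player on sight and plays an attack montage on reaching them.
; PawnSensing sets CanSeePlayer and triggers an AIMoveTo toward player 0, whose success starts the attack.
; CanAttack gates the montage for its returned duration, but is set true again on every follow call.
; Tick halts movement while CanSeePlayer is false, though nothing clears that flag once set.
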(event `self.ReceiveTick`
  (params (DeltaSeconds :type "Float (single-precision)"))
  (if (not (`self.CanSeePlayer?`))
    (`MovementComponent.StopMovementImmediately` (`self.CharacterMovement`))))

(event `self.PawnSensing.OnSeePawn`
  (params (Pawn :type "Pawn Object Reference"))
  (set `self.CanSeePlayer?` true)
  (`self.FollowPlayerCharacter`))

(event `FollowPlayerCharacter`
  (set `self.canAttack?` true)
  (if (`self.CanSeePlayer?`)
    (`|AIMoveTo` self (0.0 0.0 0.0) (`GameplayStatics.GetPlayerCharacter` 0) 50.0
      (:`OnSuccess`
        (if (`self.canAttack?`)
          (set `self.canAttack?` false)
          (bind _returnvalue (`self.PlayAnimMontage` null))
          (`KismetSystemLibrary.Delay` _returnvalue)
          (set `self.canAttack?` true))))
    (else
      (set `self.CanSeePlayer?` false))))

(fn `UserConstructionScript`)